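; Procedural rectangular arena border actor that builds a fenced perimeter from corner, pillar and border meshes at a size set in meters.
; When Generate is set, the construction script snaps the size to two-meter sections and computes four corners centered on the actor.
; It adds mesh instances along each edge with per-side yaw compensation, then fits four box colliders to the sides.
; No runtime logic runs.
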(fn `UserConstructionScript`
  (if (`self.Generate`)
    (`self.GetSizes`
      (:`NewParam`
        (`StaticMeshComponent.SetStaticMesh` (`self.cornerPillar`) (`self.CornerMesh`))
        (`StaticMeshComponent.SetStaticMesh` (`self.borderPillar`) (`self.PillarMesh`))
        (`StaticMeshComponent.SetStaticMesh` (`self.Border`) (`self.BorderMesh`))
        (`|ExecutionSequence`
          (:`then_0`
            (`self.SetCorners`))
          (:`then_1`
            (`self.SetPillars`))
          (:`then_2`
            (`self.SetBorders`))
          (:`then_3`
            (`self.SetColliders`)))))))
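; Player character Blueprint for BoS that sets up Enhanced Input and a strike ability through the Gameplay Ability System.
; BeginPlay requires a PlayerController, adds the input mapping context, and grants SimpleStrike only on a dedicated server, using the PlayerState's ability system component.
; IA_Strike calls TryActivateAbility on that component with remote activation allowed.
; Movement, debug printing and the call to the alternate SimpleStrikeToserver grant event are disconnected.
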(event `self.ReceivePossessed`
  (params (NewController :type "Controller Object Reference")))

(event `self.ReceiveTick`
  (params (DeltaSeconds :type "Float (single-precision)")))

(event `Key|LeftMouseButton`
  (params (Key :type "Key Structure")))

(event `self.ReceiveBeginPlay`
  (bind _asplayer_controller (cast `PlayerController` (`self.GetController`)))
  (`EnhancedInputSubsystemInterface.AddMappingContext` (pcsubsystem `EnhancedInputLocalPlayerSubsystem` _asplayer_controller) "/Game/BoS/Features/InputAction/BosMappingContext.BosMappingContext" 0 (struct))
  (if (`KismetSystemLibrary.IsDedicatedServer`)
    (`AbilitySystemComponent.K2_GiveAbility` (`AbilitySystemBlueprintLibrary.GetAbilitySystemComponent` (`self.PlayerState`)) "/Game/BoS/Features/BosAbilities/SimpleStrike.SimpleStrike_C" 1 -1)))

(event `SimpleStrikeToserver`
  (`AbilitySystemComponent.K2_GiveAbility` (`AbilitySystemBlueprintLibrary.GetAbilitySystemComponent` (`self.PlayerState`)) "/Game/BoS/Features/BosAbilities/SimpleStrike.SimpleStrike_C" 1 -1))

(event `EnhancedInput|/Game/BoS/Features/InputAction/IA_Strike`
  (params (ActionValue :type Boolean) (ElapsedSeconds :type "Float (double-precision)") (TriggeredSeconds :type "Float (double-precision)") (InputAction :type "InputAction Object Reference" :default "/Game/BoS/Features/InputAction/IA_Strike.IA_Strike"))
  (:`Triggered`
    (`AbilitySystemComponent.TryActivateAbility` :`self` (`AbilitySystemBlueprintLibrary.GetAbilitySystemComponent` (`self.PlayerState`)))))

(fn `UserConstructionScript`)